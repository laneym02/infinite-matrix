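; BP_Enemy is a short-lived enemy actor that removes itself through a lifespan timer set on BeginPlay.
; On overlap it casts the other actor in sequence to BP_Player and BP_Projectile.
; Player contact raises that player's Health, capped at MaxHealth, while a projectile hit increments the Score of the projectile's Player.
; Both successful casts share the same DestroyActor call, which destroys the enemy.
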(event `self.ReceiveBeginPlay`
  (`self.SetLifeSpan` 5.0))

(event `self.ReceiveActorBeginOverlap`
  (params (OtherActor :type "Actor Object Reference"))
  (`|ExecutionSequence`
    (:`then_0`
      (bind _asbp_player (cast `/Game/InfiniteMatrix/Blueprints/BP_Player` OtherActor))
      (set `/Game/InfiniteMatrix/Blueprints/BP_Player.Health` (`KismetMathLibrary.FMin` (+ (`/Game/InfiniteMatrix/Blueprints/BP_Player.Health` _asbp_player) 1.0) (`/Game/InfiniteMatrix/Blueprints/BP_Player.MaxHealth` _asbp_player)) _asbp_player))
    (:`then_1`
      (bind _asbp_projectile (cast `/Game/InfiniteMatrix/Blueprints/BP_Projectile` OtherActor))
      (bind _player (`/Game/InfiniteMatrix/Blueprints/BP_Projectile.Player` _asbp_projectile))
      (set `/Game/InfiniteMatrix/Blueprints/BP_Player.Score` (+ (`/Game/InfiniteMatrix/Blueprints/BP_Player.Score` _player) 1) _player)))
  (`self.K2_DestroyActor`))

(fn `UserConstructionScript`)